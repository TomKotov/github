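; Blinking spotlight actor that switches its light off and on a limited number of times after play begins.
; BeginPlay runs a self-looping DoN capped by Kollraz, waiting Skorost before hiding the SpotLight and Skorost2 before toggling it back on.
; The construction script calls ActiveLight to set the initial visibility from IsEnable.
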(event `self.ReceiveBeginPlay`
  (`/Engine/EditorBlueprintResources/StandardMacros.Do N` (`self.kollraz`) :!label _label
    (:`Exit`
      (`KismetSystemLibrary.Delay` (`self.skorost`))
      (`SceneComponent.SetVisibility` (`self.SpotLight`) false false)
      (`KismetSystemLibrary.Delay` (`self.skorost 2`))
      (`SceneComponent.ToggleVisibility` (`self.SpotLight`) false)
      (goto _label))))

(fn `active light`
  (params (self2 :type "SceneComponent Object Reference") (bNewVisibility :type Boolean))
  (`SceneComponent.SetVisibility` self2 bNewVisibility false))

(fn `UserConstructionScript`
  (`self.active light` (`self.SpotLight`) (`self.is enable`)))