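; An actor, named as a rolling ball, that moves along a direction and bounces off whatever blocks it, losing speed with each hit.
; Tick moves it with a swept world offset and, on a blocking hit, reflects the direction about the hit normal's X and Y.
; Each bounce subtracts a fixed step, taken as a tenth of the starting speed at BeginPlay, until a minimum speed is reached.
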(event `self.ReceiveBeginPlay`
  (set `self.kofic` (* (`self.start speed`) 0.1)))

(event `self.ReceiveTick`
  (params (DeltaSeconds :type "Float (single-precision)"))
  (bind _sweephitresult (`self.K2_AddActorWorldOffset` (* (* (`self.direction `) (`self.start speed`)) DeltaSeconds) true))
  (bind (_bblockinghit _binitialoverlap _time _distance _location _impactpoint _normal) (`GameplayStatics.BreakHitResult` _sweephitresult))
  (if _bblockinghit
    (set `self.direction ` (`KismetMathLibrary.GetReflectionVector` (`self.direction `) (`KismetMathLibrary.MakeVector` (.x _normal) (.y _normal))))
    (set `self.start speed` (`KismetMathLibrary.FMax` (- (`self.start speed`) (`self.kofic`)) (`self.minspeed`)))))

(fn `UserConstructionScript`)